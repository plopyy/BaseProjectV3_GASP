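; Animation modifier that bakes an orientation warping alpha curve from whether the root motion is going straight or turning.
; It samples the root bone at a fixed rate, comparing per-sample changes in rotation and travel direction against angle thresholds.
; Straight/turn transitions become paired 0/1 keys, offset to blend in before turns and out after them, with optional inversion.
; Reverting optionally removes the curve.
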(event EventOnApply
  (params (AnimationSequence :type Anim%20Sequence%20Object%20Reference))
  (CallFunction|InitIterationParams AnimationSequence)
  (Class|AnimationBlueprintLibrary|AddCurve (Variables|Default|GetTargetAnim) (Variables|Default|GetCurveName) "RCT_Float" false)
  (while (< (+ (Variables|Default|GetSampleTime) 1e-05) (Animation|GetPlayLength (Variables|Default|GetTargetAnim)))
    ;[1 1 1] Get current sample info
    (Variables|Default|SetSampleTime (CallFunction|GetCurrentSampleTime))
    (bind _result (Math|Integer|IncrementInt (Variables|Default|GetSampleIndex))
      (:%20%20
        (Variables|Default|SetSampleIndex _result)
        (Variables|Default|SetBoneTransform (Class|AnimationBlueprintLibrary|GetBonePoseforTime (Variables|Default|GetTargetAnim) "root" (Variables|Default|GetSampleTime) false))
        (Utilities|FlowControl|Sequence
          (:then_0
            (if (> (Variables|Default|GetSampleIndex) 1)
              (Utilities|FlowControl|Sequence
                (:then_0
                  (if (not (Math|Vector|VectorIsNearlyZero (Math|Vector|Normalize (- (.location (Variables|Default|GetBoneTransform)) (.location (Variables|Default|GetLastBoneTransform)))) 0.001))
                    (Variables|Default|SetRootMotionTranslationAngle (Math|Rotator|MakeRotfromX (Math|Vector|Normalize (- (.location (Variables|Default|GetBoneTransform)) (.location (Variables|Default|GetLastBoneTransform))))))))
                (:then_1
                  (if (> (Variables|Default|GetSampleIndex) 2)
                    (Utilities|FlowControl|Sequence
                      (:then_1
                        (Variables|Default|SetRotationError (+ (Variables|Default|GetRotationError) (Math|Float|Max(Float) (Math|Float|Absolute(Float) (.roll (Math|Rotator|Delta(Rotator) (.rotation (Variables|Default|GetLastBoneTransform)) (.rotation (Variables|Default|GetBoneTransform))))) (Math|Float|Absolute(Float) (.pitch (Math|Rotator|Delta(Rotator) (.rotation (Variables|Default|GetLastBoneTransform)) (.rotation (Variables|Default|GetBoneTransform))))) (Math|Float|Absolute(Float) (.yaw (Math|Rotator|Delta(Rotator) (.rotation (Variables|Default|GetLastBoneTransform)) (.rotation (Variables|Default|GetBoneTransform))))))))
                        (Variables|Default|SetTranslationError (+ (Variables|Default|GetTranslationError) (Math|Float|Max(Float) (Math|Float|Absolute(Float) (.roll (Math|Rotator|Delta(Rotator) (Variables|Default|GetLastRootMotionTranslationAngle) (Variables|Default|GetRootMotionTranslationAngle)))) (Math|Float|Absolute(Float) (.pitch (Math|Rotator|Delta(Rotator) (Variables|Default|GetLastRootMotionTranslationAngle) (Variables|Default|GetRootMotionTranslationAngle)))) (Math|Float|Absolute(Float) (.yaw (Math|Rotator|Delta(Rotator) (Variables|Default|GetLastRootMotionTranslationAngle) (Variables|Default|GetRootMotionTranslationAngle)))))))
                        (Variables|Default|SetbGoingStraight (and (< (Variables|Default|GetRotationError) (Variables|Default|GetRotationAngleThreshold)) (< (Variables|Default|GetTranslationError) (Variables|Default|GetTranslationAngleThreshold)))))
                      (:then_2
                        (if (== (Variables|Default|GetSampleIndex) 4)
                          (Class|AnimationBlueprintLibrary|AddFloatCurveKey (Variables|Default|GetTargetAnim) (Variables|Default|GetCurveName) (Variables|Default|GetSampleTime) (Math|Conversions|ToFloat(Boolean) (Class|KismetMathLibrary|XORBoolean (Variables|Default|GetbGoingStraight) (Variables|Default|GetbInvert))))))
                      (:then_3
                        (if (and (!= (Variables|Default|GetbGoingStraight) (Variables|Default|GetbLastGoingStraight)) (> (Variables|Default|GetSampleIndex) 3))
                          (Class|AnimationBlueprintLibrary|AddFloatCurveKey (Variables|Default|GetTargetAnim) (Variables|Default|GetCurveName) (- (Variables|Default|GetSampleTime) (Math|Float|SelectFloat 0.0 (Variables|Default|GetBlendInTime) (Variables|Default|GetbGoingStraight))) (Math|Float|SelectFloat 1.0 0.0 (Class|KismetMathLibrary|XORBoolean (Variables|Default|GetbLastGoingStraight) (Variables|Default|GetbInvert))))
                          (Class|AnimationBlueprintLibrary|AddFloatCurveKey (Variables|Default|GetTargetAnim) (Variables|Default|GetCurveName) (+ (Variables|Default|GetSampleTime) (Math|Float|SelectFloat (Variables|Default|GetBlendOutTime) 0.0 (Variables|Default|GetbGoingStraight))) (Math|Float|SelectFloat 1.0 0.0 (Class|KismetMathLibrary|XORBoolean (Variables|Default|GetbGoingStraight) (Variables|Default|GetbInvert))))))))))))
          (:then_1
            (Variables|Default|SetbLastGoingStraight (Variables|Default|GetbGoingStraight))
            (Variables|Default|SetLastBoneTransform (Variables|Default|GetBoneTransform))
            (Variables|Default|SetLastRootMotionTranslationAngle (Variables|Default|GetRootMotionTranslationAngle))
            (Variables|Default|SetRotationError 0.0)
            (Variables|Default|SetTranslationError 0.0)))))))

(event EventOnRevert
  (params (AnimationSequence :type Anim%20Sequence%20Object%20Reference))
  (if (Variables|Default|GetbDeleteCurveOnRevert)
    (Class|AnimationBlueprintLibrary|RemoveCurve AnimationSequence (Variables|Default|GetCurveName) false)))

(fn InitIterationParams
  (params (InTargetAnim :type Anim%20Sequence%20Base%20Object%20Reference))
  (bind _returnvalue (Math|Transform|MakeTransform "0, 0, 0"))
  (Variables|Default|SetTargetAnim InTargetAnim)
  (Variables|Default|SetTimePerSample (/ 1.0 (Math|Conversions|ToFloat(Integer) (Variables|Default|GetSamplesPerSecond))))
  (Variables|Default|SetSampleTime 0.0)
  (Variables|Default|SetSampleIndex 0)
  (Variables|Default|SetLastBoneTransform _returnvalue)
  (Variables|Default|SetBoneTransform _returnvalue))

(fn GetCurrentSampleTime
  (return (Math|Float|Clamp(Float) (* (Variables|Default|GetSampleIndex) (Variables|Default|GetTimePerSample)) 0.0 (Animation|GetPlayLength (Variables|Default|GetTargetAnim)))))