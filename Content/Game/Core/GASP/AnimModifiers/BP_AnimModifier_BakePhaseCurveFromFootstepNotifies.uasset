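; Animation modifier that rebuilds a float "Phase" curve on an animation sequence from left and right footstep notify tracks.
; Each left step keys 1 and each right step keys 0, with a constant -1 key just before left steps, forming a descending wrapping ramp.
; Boundary keys wrap by sequence length when looping; otherwise they extrapolate from step spacing, or start at time zero with StartAt0.
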(event EventOnApply
  (params (AnimationSequence :type Anim%20Sequence%20Object%20Reference))
  (bind _output_get (Variables|Default|SetAnimation%20Sequence AnimationSequence))
  (CallFunction|ClearCurve _output_get "Phase")
  (Utilities|FlowControl|Sequence
    (:then_0
      (bind _output_get_2 (Variables|Default|SetLeftFootEvents (Class|AnimationBlueprintLibrary|GetAnimationNotifyEventsforTrack (Variables|Default|GetAnimation%20Sequence) (Variables|Default|GetLeftFootTrack))))
      (for _array_element _output_get_2
        (CallFunction|AddKey (Variables|Default|GetAnimation%20Sequence) (Class|AnimationBlueprintLibrary|GetAnimNotifyEventTriggerTime _array_element) (Variables|Default|GetName) (Variables|Default|GetLeftPhaseTransform) true)))
    (:then_1
      (bind _output_get_3 (Variables|Default|SetRightFootEvents (Class|AnimationBlueprintLibrary|GetAnimationNotifyEventsforTrack (Variables|Default|GetAnimation%20Sequence) (Variables|Default|GetRightFootTrack))))
      (for _array_element_2 _output_get_3
        (CallFunction|AddKey (Variables|Default|GetAnimation%20Sequence) (Class|AnimationBlueprintLibrary|GetAnimNotifyEventTriggerTime _array_element_2) (Variables|Default|GetName) (Variables|Default|GetRightPhaseTransform) false)))
    (:then_2
      (Variables|Default|SetLeftFirst (< (Class|AnimationBlueprintLibrary|GetAnimNotifyEventTriggerTime (Utilities|Array|Get(acopy) (Variables|Default|GetLeftFootEvents))) (Class|AnimationBlueprintLibrary|GetAnimNotifyEventTriggerTime (Utilities|Array|Get(acopy) (Variables|Default|GetRightFootEvents)))))
      (Variables|Default|SetLeftLast (> (Class|AnimationBlueprintLibrary|GetAnimNotifyEventTriggerTime (Utilities|Array|Get(acopy) (Variables|Default|GetLeftFootEvents) (Utilities|Array|LastIndex (Variables|Default|GetLeftFootEvents)))) (Class|AnimationBlueprintLibrary|GetAnimNotifyEventTriggerTime (Utilities|Array|Get(acopy) (Variables|Default|GetRightFootEvents) (Utilities|Array|LastIndex (Variables|Default|GetRightFootEvents)))))))
    (:then_3
      (if (Variables|Default|GetLooping)
        (CallFunction|AddKey (Variables|Default|GetAnimation%20Sequence) (- (Class|AnimationBlueprintLibrary|GetAnimNotifyEventTriggerTime (Utilities|Array|Get(acopy) (select (Variables|Default|GetLeftFirst) (Variables|Default|GetRightFootEvents) (Variables|Default|GetLeftFootEvents)) (Utilities|Array|LastIndex (select (Variables|Default|GetLeftFirst) (Variables|Default|GetRightFootEvents) (Variables|Default|GetLeftFootEvents))))) (Class|AnimationBlueprintLibrary|GetSequenceLength (Variables|Default|GetAnimation%20Sequence))) (Variables|Default|GetName) (select (Variables|Default|GetLeftFirst) (Variables|Default|GetRightPhaseTransform) (Variables|Default|GetLeftPhaseTransform)) (select (Variables|Default|GetLeftFirst) false true))
        (CallFunction|AddKey (Variables|Default|GetAnimation%20Sequence) (+ (Class|AnimationBlueprintLibrary|GetAnimNotifyEventTriggerTime (Utilities|Array|Get(acopy) (select (Variables|Default|GetLeftLast) (Variables|Default|GetRightFootEvents) (Variables|Default|GetLeftFootEvents)))) (Class|AnimationBlueprintLibrary|GetSequenceLength (Variables|Default|GetAnimation%20Sequence))) (Variables|Default|GetName) (select (Variables|Default|GetLeftLast) (Variables|Default|GetRightPhaseTransform) (Variables|Default|GetLeftPhaseTransform)) (select (Variables|Default|GetLeftLast) false true))
        (else
          (if (Variables|Default|GetStartAt0)
            (CallFunction|AddKey (Variables|Default|GetAnimation%20Sequence) 0.0 (Variables|Default|GetName) (Math|Transform|MakeTransform "0, 0, 0" (select (Variables|Default|GetLeftFirst) (.rotation (Variables|Default|GetRightPhaseTransform)) (.rotation (Variables|Default|GetLeftPhaseTransform))) "1.000000,1.000000,1.000000") (select (Variables|Default|GetLeftFirst) false true))
            (else
              (CallFunction|AddKey (Variables|Default|GetAnimation%20Sequence) (- (Class|AnimationBlueprintLibrary|GetAnimNotifyEventTriggerTime (Utilities|Array|Get(acopy) (select (Variables|Default|GetLeftFirst) (Variables|Default|GetLeftFootEvents) (Variables|Default|GetRightFootEvents)))) (- (Class|AnimationBlueprintLibrary|GetAnimNotifyEventTriggerTime (Utilities|Array|Get(acopy) (select (Variables|Default|GetLeftFirst) (Variables|Default|GetRightFootEvents) (Variables|Default|GetLeftFootEvents)))) (Class|AnimationBlueprintLibrary|GetAnimNotifyEventTriggerTime (Utilities|Array|Get(acopy) (select (Variables|Default|GetLeftFirst) (Variables|Default|GetLeftFootEvents) (Variables|Default|GetRightFootEvents)))))) (Variables|Default|GetName) (select (Variables|Default|GetLeftFirst) (Variables|Default|GetRightPhaseTransform) (Variables|Default|GetLeftPhaseTransform)) (select (Variables|Default|GetLeftFirst) false true))))
          (CallFunction|AddKey (Variables|Default|GetAnimation%20Sequence) (+ (Class|AnimationBlueprintLibrary|GetAnimNotifyEventTriggerTime (Utilities|Array|Get(acopy) (select (Variables|Default|GetLeftLast) (Variables|Default|GetLeftFootEvents) (Variables|Default|GetRightFootEvents)) (Utilities|Array|LastIndex (select (Variables|Default|GetLeftLast) (Variables|Default|GetLeftFootEvents) (Variables|Default|GetRightFootEvents))))) (- (Class|AnimationBlueprintLibrary|GetAnimNotifyEventTriggerTime (Utilities|Array|Get(acopy) (select (Variables|Default|GetLeftLast) (Variables|Default|GetLeftFootEvents) (Variables|Default|GetRightFootEvents)) (Utilities|Array|LastIndex (select (Variables|Default|GetLeftLast) (Variables|Default|GetLeftFootEvents) (Variables|Default|GetRightFootEvents))))) (Class|AnimationBlueprintLibrary|GetAnimNotifyEventTriggerTime (Utilities|Array|Get(acopy) (select (Variables|Default|GetLeftLast) (Variables|Default|GetRightFootEvents) (Variables|Default|GetLeftFootEvents)) (Utilities|Array|LastIndex (select (Variables|Default|GetLeftLast) (Variables|Default|GetRightFootEvents) (Variables|Default|GetLeftFootEvents))))))) (Variables|Default|GetName) (select (Variables|Default|GetLeftLast) (Variables|Default|GetRightPhaseTransform) (Variables|Default|GetLeftPhaseTransform)) (select (Variables|Default|GetLeftLast) false true)))))))

(fn AddKey
  (params (AnimationSequenceBase :type Anim%20Sequence%20Base%20Object%20Reference) (Time :type Float%20%28single-precision%29) (CurveName :type Name) (Transform :type Transform%20%28by%20ref%29) (IsLeft :type Boolean))
  (bind _curveb (LocalVariables|GetCurveB))
  (bind _controller (Variables|/Script/Engine.AnimSequenceBase|GetController AnimationSequenceBase))
  (Class|AnimationCurveIdentifierExtensions|SetCurveIdentifier _curveb "Phase" "RCT_Float")
  (Class|AnimationDataController|SetCurveKey _controller _curveb (Utilities|Struct|MakeRichCurveKey "RCIM_Linear" "RCTM_Auto" "RCTWM_WeightedNone" Time (Math|Float|SelectFloat 1.0 0.0 IsLeft)) true)
  (if IsLeft
    (Class|AnimationDataController|SetCurveKey _controller _curveb (Utilities|Struct|MakeRichCurveKey "RCIM_Constant" "RCTM_Auto" "RCTWM_WeightedNone" (- Time 0.01) -1.0) true)))

(fn ClearCurve
  (params (AnimationSequenceBase :type Anim%20Sequence%20Base%20Object%20Reference) (CurveName :type Name))
  (bind _returnvalue (Class|AnimationBlueprintLibrary|DoesCurveExist AnimationSequenceBase CurveName "RCT_Float"))
  (if _returnvalue
    (Class|AnimationBlueprintLibrary|RemoveCurve (Variables|Default|GetAnimation%20Sequence) CurveName false))
  (Class|AnimationBlueprintLibrary|AddCurve AnimationSequenceBase CurveName "RCT_Float" false))