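; Traversal component that computes front and back ledge locations and normals from an initial obstacle hit and writes them into the traversal check struct.
; It nudges the hit toward the object's center, shifts it away from nearby corners and width-checks narrow faces such as cylinders.
; Component-only line traces along the hit plane find the front edge, and a reverse trace finds the back face and its ledge.
; Object up is flipped to match the owner's, supporting upside-down objects.
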(fn TryandCalculateLedges
  (params (InitialHitResult :type Hit%20Result%20Structure%20%28by%20ref%29) (TraversalCheckStuct :type Struct%20Traversal%20Check%20Result%20Structure%20%28by%20ref%29))
  (bind (_found_front_ledge _start_ledge_location _start_ledge_normal _foundbackledge _end_ledge_location _end_ledge_normal) (CallFunction|ComputeLedgeData InitialHitResult (Transformation|GetActorForwardVector (Components|GetOwner))))
  (Utilities|Struct|SetmembersinStruct_TraversalCheckResult TraversalCheckStuct _found_front_ledge _start_ledge_location _start_ledge_normal _foundbackledge _end_ledge_location _end_ledge_normal))

(fn ComputeLedgeData
  (params (HitResult :type Hit%20Result%20Structure%20%28by%20ref%29) (PlayerDirection :type Vector))
  (bind _hitcomponent (Collision|BreakHitResult HitResult))
  (bind (_bblockinghit _binitialoverlap _time _distance _location _impactpoint _normal _impactnormal _physmat _hitactor _hitcomponent_2) (Collision|BreakHitResult HitResult))
  (bind (_bblockinghit_2 _binitialoverlap_2 _time_2 _distance_2 _location_2 _impactpoint_2 _normal_2 _impactnormal_2 _physmat_2 _hitactor_2 _hitcomponent_3) (Collision|BreakHitResult HitResult))
  (bind _returnvalue (Math|Vector|GetUpVector _hitcomponent))
  (CallFunction|NudgeTraceTowardsObjectOrigin HitResult)
  (LocalVariables|SetStartNormal _impactnormal)
  (LocalVariables|SetTraceLenght (* (.SphereRadius (Collision|GetComponentBounds _hitcomponent_2)) 2.0))
  (LocalVariables|SetAbsoluteObjectUpVector (* _returnvalue (Math|Float|Sign(Float) (Math|Vector|DotProduct _returnvalue (Transformation|GetActorUpVector (Components|GetOwner))))))
  (Utilities|FlowControl|Sequence
    (:then_0
      ;[1 1 1] 1. Offset the trace towards the opposite direction of corners, by the half ledge width, ensuring we arent grabbing the air if we are close to a corner
      (Utilities|FlowControl|Sequence
        (:then_0
          (bind (_ofsettedcornerpoint _closetocorner _distancetocorner) (CallFunction|TraceCorners HitResult (Math|Vector|CrossProduct (.ImpactNormal (Collision|BreakHitResult HitResult)) (LocalVariables|GetAbsoluteObjectUpVector)) (LocalVariables|GetTraceLenght)))
          (LocalVariables|SetRightEdgeDistance _distancetocorner)
          (if _closetocorner
            (CallFunction|SetTraceHitPoint HitResult _ofsettedcornerpoint)))
        (:then_1
          (bind (_ofsettedcornerpoint_2 _closetocorner_2 _distancetocorner_2) (CallFunction|TraceCorners HitResult (Math|Vector|CrossProduct (LocalVariables|GetAbsoluteObjectUpVector) (.ImpactNormal (Collision|BreakHitResult HitResult))) (LocalVariables|GetTraceLenght)))
          (if _closetocorner_2
            (if (< (+ _distancetocorner_2 (LocalVariables|GetRightEdgeDistance)) (Variables|Default|GetMin%20Ledge%20Width))
              ;[1 1 1] If the corners of the current hit plane are too close together, it doesnt necessarely mean we cant traverse this object, so we should try and see if we'll hit the object with our width params left and right.
              ; A cylinder is a good example of a shape which will reach this code.
              (bind _returnvalue_2 (CallFunction|TraceWidth HitResult (Math|Vector|CrossProduct (LocalVariables|GetAbsoluteObjectUpVector) (.ImpactNormal (Collision|BreakHitResult HitResult)))))
              (if _returnvalue_2
                (bind _returnvalue_3 (CallFunction|TraceWidth HitResult (Math|Vector|NegateVector (Math|Vector|CrossProduct (LocalVariables|GetAbsoluteObjectUpVector) (.ImpactNormal (Collision|BreakHitResult HitResult))))))
                (if (not _returnvalue_3)
                  (return false "0, 0, 0" "0, 0, 0" false "0, 0, 0" "0, 0, 0"))
                (else
                  (return false "0, 0, 0" "0, 0, 0" false "0, 0, 0" "0, 0, 0")))
              (else
                (CallFunction|SetTraceHitPoint HitResult _ofsettedcornerpoint_2)))))))
    (:then_1
      ;[1 1 1] 2. Given our initial hit, check for an edge by tracing towards the hit point, along the plane
      (bind (_outhit _returnvalue_4) (CallFunction|TraceAlongHitPlane HitResult (LocalVariables|GetTraceLenght) (LocalVariables|GetAbsoluteObjectUpVector)))
      (if _returnvalue_4
        (bind _output_get (LocalVariables|SetStart%20Ledge (.ImpactPoint (Collision|BreakHitResult _outhit))))
        (if (Variables|Default|GetPersistent%20Show%20Trace)
          (Rendering|Debug|DrawDebugSphere _output_get 1e+01 12 "(R=0.042591,G=1.000000,B=0.000000,A=1.000000)" 32131231.0))
        (else
          (return false "0, 0, 0" "0, 0, 0" false "0, 0, 0" "0, 0, 0"))))
    (:then_2
      ;[1 1 1] 3. Reverse our trace to figure out the penetrating point of the backface of the object
      (bind (_hitlocation _hitnormal _bonename _outhit_2 _returnvalue_5) (Collision|LineTraceComponent _hitcomponent_3 (- _impactpoint_2 (* _impactnormal_2 (LocalVariables|GetTraceLenght))) _impactpoint_2 (Variables|Default|GetTrace%20Complex) (Variables|Default|GetShow%20Trace) (Variables|Default|GetPersistent%20Show%20Trace)))
      ;[1 1 1] If we've found a hit from our backface trace, try to find the ledge by tracing along the hit plane from above
      (bind _output_get_2 (LocalVariables|SetHasBackLedge _returnvalue_5))
      (if _output_get_2
        (LocalVariables|SetEndNormal _hitnormal)
        (bind _outhit_3 (CallFunction|TraceAlongHitPlane _outhit_2 (LocalVariables|GetTraceLenght) (LocalVariables|GetAbsoluteObjectUpVector)))
        (bind _output_get_3 (LocalVariables|SetEndLedge (.ImpactPoint (Collision|BreakHitResult _outhit_3))))
        (if (Variables|Default|GetPersistent%20Show%20Trace)
          (Rendering|Debug|DrawDebugSphere _output_get_3 1e+01 12 "(R=0.000000,G=1.000000,B=0.912636,A=1.000000)" 32131231.0))))
    (:then_3
      (return true (LocalVariables|GetStart%20Ledge) (LocalVariables|GetStartNormal) (LocalVariables|GetHasBackLedge) (LocalVariables|GetEndLedge) (LocalVariables|GetEndNormal)))))

(fn TraceAlongHitPlane
  (params (Hit :type Hit%20Result%20Structure%20%28by%20ref%29) (TraceLenght :type Float%20%28single-precision%29) (TraceDirection :type Vector))
  (bind _impactnormal (Collision|BreakHitResult Hit))
  (bind _returnvalue (Math|Vector|CrossProduct _impactnormal TraceDirection))
  (bind (_bblockinghit _binitialoverlap _time _distance _location _impactpoint _normal _impactnormal_2 _physmat _hitactor _hitcomponent) (Collision|BreakHitResult Hit))
  (bind _returnvalue_2 (Math|Vector|CrossProduct _returnvalue _impactnormal))
  (bind _returnvalue_3 (- _impactpoint _impactnormal_2))
  (bind _returnvalue_4 (Math|Vector|Normalize _returnvalue_2))
  (bind _returnvalue_5 (* TraceLenght _returnvalue_4))
  (bind _returnvalue_6 (+ _returnvalue_5 _returnvalue_3))
  (bind (_hitlocation _hitnormal _bonename _outhit _returnvalue_7) (Collision|LineTraceComponent _hitcomponent _returnvalue_6 (Math|Vector|Lerp(Vector) _returnvalue_6 _returnvalue_3 1.5) (Variables|Default|GetTrace%20Complex) (Variables|Default|GetShow%20Trace) (Variables|Default|GetPersistent%20Show%20Trace)))
  (return _outhit _returnvalue_7))

(fn NudgeTraceTowardsObjectOrigin
  (params (HitResult :type Hit%20Result%20Structure%20%28by%20ref%29))
  (bind (_bblockinghit _binitialoverlap _time _distance _location _impactpoint _normal _impactnormal _physmat _hitactor _hitcomponent _hitbonename _bonename _hititem _elementindex _faceindex _tracestart _traceend) (Collision|BreakHitResult HitResult))
  (|SetBy-RefVar HitResult (Collision|MakeHitResult _bblockinghit _binitialoverlap _time _distance _location (- _impactpoint (Math|Vector|GetUnitDirection(Vector) (Class|KismetMathLibrary|ProjectPointontoPlane (.Origin (Collision|GetComponentBounds _hitcomponent)) _impactpoint _impactnormal) _impactpoint)) _normal _impactnormal _physmat _hitactor _hitcomponent _hitbonename _bonename _hititem _elementindex _faceindex _tracestart _traceend)))

(fn SetTraceHitPoint
  (params (HitResult :type Hit%20Result%20Structure%20%28by%20ref%29) (New%20Impact%20Point :type Vector))
  (bind (_bblockinghit _binitialoverlap _time _distance _location _impactpoint _normal _impactnormal _physmat _hitactor _hitcomponent _hitbonename _bonename _hititem _elementindex _faceindex _tracestart _traceend) (Collision|BreakHitResult HitResult))
  (|SetBy-RefVar HitResult (Collision|MakeHitResult _bblockinghit _binitialoverlap _time _distance _location New%20Impact%20Point _normal _impactnormal _physmat _hitactor _hitcomponent _hitbonename _bonename _hititem _elementindex _faceindex _tracestart _traceend)))

(fn TraceCorners
  (params (Hit :type Hit%20Result%20Structure%20%28by%20ref%29) (TraceDirection :type Vector) (TraceLenght :type Float%20%28single-precision%29))
  (bind (_outhit _returnvalue) (CallFunction|TraceAlongHitPlane Hit TraceLenght TraceDirection))
  (if _returnvalue
    (return (+ (.ImpactPoint (Collision|BreakHitResult _outhit)) (* (Math|Vector|NegateVector TraceDirection) (/ (Variables|Default|GetMin%20Ledge%20Width) 2.0))) (< (Math|Vector|Distance(Vector) (.ImpactPoint (Collision|BreakHitResult _outhit)) (.ImpactPoint (Collision|BreakHitResult Hit))) (/ (Variables|Default|GetMin%20Ledge%20Width) 2.0)) (Math|Vector|Distance(Vector) (.ImpactPoint (Collision|BreakHitResult _outhit)) (.ImpactPoint (Collision|BreakHitResult Hit))))
    (else
      (return "0, 0, 0" false 0.0))))

(fn TraceWidth
  (params (Hit :type Hit%20Result%20Structure%20%28by%20ref%29) (Direction :type Vector))
  (bind (_bblockinghit _binitialoverlap _time _distance _location _impactpoint _normal _impactnormal _physmat _hitactor _hitcomponent) (Collision|BreakHitResult Hit))
  (bind _min_front_ledge_depth (Variables|Default|GetMin%20Front%20Ledge%20Depth))
  (bind _min_ledge_width (Variables|Default|GetMin%20Ledge%20Width))
  (bind _returnvalue (/ _min_ledge_width 2.0))
  (bind _returnvalue_2 (* _impactnormal _min_front_ledge_depth))
  (bind _returnvalue_3 (* Direction _returnvalue))
  (bind _returnvalue_4 (+ _impactpoint _returnvalue_3))
  (bind _returnvalue_5 (Collision|LineTraceComponent _hitcomponent (+ _returnvalue_4 _returnvalue_2) (- _returnvalue_4 _returnvalue_2) (Variables|Default|GetTrace%20Complex) (Variables|Default|GetShow%20Trace) (Variables|Default|GetPersistent%20Show%20Trace)))
  (return _returnvalue_5))